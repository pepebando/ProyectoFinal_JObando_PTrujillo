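; Game mode for a Missile Command game that drives enemy missile spawning from four sides: rear, front, right and left.
; On BeginPlay it finds the first actor of each spawner class and starts a looping timer on its Evento_SpawnMisil, at EnemyPS per second.
; Tick, gated by a five-second Delay, sets IContadoRandomColor through ElegirUnRandomArreglo, whose random-pick nodes are left unconnected.
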(event Custom|LlamarSpawn1
  ;[1 1 1] LlamaSpawnClase1EnUnRangoDeTiempo
  (bind _outactors (Actor|GetAllActorsOfClass "/Game/FirstPersonBP/Misiles/SpawnClassMisil1Trasera.SpawnClassMisil1Trasera_C"))
  (bind _output_get (Variables|Default|SetVar_Spawn1 (Utilities|Array|Get(acopy) _outactors)))
  (Utilities|Time|SetTimerbyFunctionName _output_get "Evento_SpawnMisil" (/ 1.0 (Variables|Default|GetEnemyPS)) true))

(event Custom|LlamarSpawn2
  ;[1 1 1] LlamaSpawnClase2EnUnRangoDeTiempo
  (bind _outactors (Actor|GetAllActorsOfClass "/Game/FirstPersonBP/Misiles/SpawnClassMisil2Frontal.SpawnClassMisil2Frontal_C"))
  (bind _output_get (Variables|Default|SetVar_Spawn2 (Utilities|Array|Get(acopy) _outactors)))
  (Utilities|Time|SetTimerbyFunctionName _output_get "Evento_SpawnMisil" (/ 1.0 (Variables|Default|GetEnemyPS)) true))

(event Custom|LlamarSpawn4
  ;[1 1 1] LlamaSpawnClase4EnUnRangoDeTiempo
  (bind _outactors (Actor|GetAllActorsOfClass "/Game/FirstPersonBP/Misiles/SpawnClassMisil4Izquierda.SpawnClassMisil4Izquierda_C"))
  (bind _output_get (Variables|Default|SetVar_Spawn4 (Utilities|Array|Get(acopy) _outactors)))
  (Utilities|Time|SetTimerbyFunctionName _output_get "Evento_SpawnMisil" (/ 1.0 (Variables|Default|GetEnemyPS)) true))

(event Custom|LlamarSpawn3
  ;[1 1 1] LlamaSpawnClase3EnUnRangoDeTiempo
  (bind _outactors (Actor|GetAllActorsOfClass "/Game/FirstPersonBP/Misiles/SpawnClassMisil3Derecha.SpawnClassMisil3Derecha_C"))
  (bind _output_get (Variables|Default|SetVar_Spawn3 (Utilities|Array|Get(acopy) _outactors)))
  (Utilities|Time|SetTimerbyFunctionName _output_get "Evento_SpawnMisil" (/ 1.0 (Variables|Default|GetEnemyPS)) true))

(event EventTick
  (params (DeltaSeconds :type Float%20%28single-precision%29))
  ;[1 1 1] EjecucionLlamadas
  (Utilities|FlowControl|Delay 5.0)
  (Variables|Default|Seti_ContadoRandomColor (.Index (Utilities|ElegirUnRandomArreglo (Utilities|Array|MakeArray 0 1 2 3)))))

(event EventBeginPlay
  ;[1 1 1] LlamadoDeSpawns
  (CallFunction|LlamarSpawn1)
  (CallFunction|LlamarSpawn2)
  (CallFunction|LlamarSpawn3)
  (CallFunction|LlamarSpawn4))

(fn ConstructionScript)